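; BP_BaseEnemyController is the AI controller for enemies, running BT_Enemy on possession and activating AI perception at begin play.
; When perception senses an actor other than a BaseEnemy, it stores it in the player blackboard key.
; Losing a stimulus from any actor tells the controlled BaseEnemy to return to spawn, without clearing that key.
; A SetCanAttack event writes the attack permission flag to the blackboard.
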(event OnTargetPerceptionUpdated(AIPerception)
  (params (Actor :type Actor%20Object%20Reference) (Stimulus :type AI%20Stimulus%20Structure))
  (if (.bSuccessfullySensed (Utilities|Struct|BreakAIStimulus Stimulus))
    (Utilities|Casting|CastToBaseEnemy Actor
      (:CastFailed
        (AI|Components|Blackboard|SetValueasObject (Variables|Default|GetBlackboard) (Variables|Default|GetPlayerVariableName) Actor)))
    (else
      (bind _asbase_enemy (Utilities|Casting|CastToBaseEnemy (Pawn|GetControlledPawn)))
      (Class|BaseEnemy|GoBacktoSpawn _asbase_enemy))))

(event EventBeginPlay
  (Components|Activation|Activate (Variables|Default|GetAIPerception) false))

(event EventTick
  (params (DeltaSeconds :type Float%20%28single-precision%29)))

(event EventPossess
  (params (PossessedPawn :type Pawn%20Object%20Reference))
  (AI|RunBehaviorTree "/Game/Enemies/BT_Enemy.BT_Enemy"))

(event EventSetCanAttack
  (params (CanAttack :type Boolean))
  (AI|Components|Blackboard|SetValueasBool (Variables|Default|GetBlackboard) (Variables|Default|GetCanAttackVariableName) CanAttack))

(fn ConstructionScript)